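; BP_PathBuilder turns GPS tracking rows from a data table into a linear spline path for one tracked individual.
; At construction it takes a chosen reference row as origin, then filters rows by Identifier.
; GPStoPosition maps longitude and latitude to flat X/Y offsets from that origin, scaled by PositionScale, for world-space spline points.
; Alongside each point it appends a TimeTable timespan holding only the timestamp's hour, and updates the spline once afterward.
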(event `self.ReceiveBeginPlay`)

(fn `GPStoPosition`
  (params (Entry :type "/Game/S_PenguinGPS Structure (by ref)"))
  (returns (Position :type "Vector Structure"))
  (bind (_timestamp _location_long _location_lat) (break `/Game/S_PenguinGPS` Entry))
  (return (* (- (`KismetMathLibrary.MakeVector` _location_long _location_lat 0.0) (`self.PositionReference`)) (`self.PositionScale`))))

(fn `UserConstructionScript`
  (locals (TableNames :type "Array of Name"))
  (bind _spline (`self.Spline`))
  (`|ExecutionSequence`
    (:`then_0`
      ;[1 1 1] Get Reference Position
      (bind _outrownames (`DataTableFunctionLibrary.GetDataTableRowNames` (`self.DataTable`)))
      (bind _output_get (set `local.TableNames` _outrownames))
      (bind _returnvalue (`|GetDataTableRow` (`self.DataTable`) (`|GetArrayItem` _output_get (`self.ReferenceRow`)))
        (:`then`
          (bind (_timestamp _location_long _location_lat) (break `/Game/S_PenguinGPS` _returnvalue))
          (set `self.PositionReference` (`KismetMathLibrary.MakeVector` _location_long _location_lat 0.0)))))
    (:`then_1`
      (for _index (range (+ (`KismetArrayLibrary.Array_Length` (`local.TableNames`)) 1))
        (bind _returnvalue_2 (`|GetDataTableRow` (`self.DataTable`) (`|GetArrayItem` (`local.TableNames`) _index))
          (:`then`
            (if (== (`.individual-local-identifier_12_9AC8A2A14EFFF01C7A5292B27DF39373` (break `/Game/S_PenguinGPS` _returnvalue_2)) (`self.Identifier`))
              (bind _position (`self.GPStoPosition` _returnvalue_2))
              (`SplineComponent.AddSplinePoint` _spline _position "World" false)
              (`SplineComponent.SetSplinePointType` _spline (- (`SplineComponent.GetNumberOfSplinePoints` _spline) 1) "Linear" false)
              (`KismetArrayLibrary.Array_Add` (`self.TimeTable`) (`KismetMathLibrary.MakeTimespan` 0 (`KismetStringLibrary.Conv_StringToInt` (`KismetStringLibrary.GetSubstring` (`.timestamp_2_E110F35C45A022D96023FF903F24989F` (break `/Game/S_PenguinGPS` _returnvalue_2)) 11 2)))))))))
    (:`then_2`
      (`SplineComponent.UpdateSpline` (`self.Spline`)))))