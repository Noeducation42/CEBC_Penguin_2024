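; Path manager actor that turns GPS tracking data from a data table into penguin paths.
; The construction script groups all rows, or an index range, by individual ID, converting longitude and latitude into scaled positions relative to a reference row.
; On BeginPlay, it spawns a BP_PathEntity with those coordinates for each selected individual, plus a BP_Penguin linked to that path.
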(event `self.ReceiveBeginPlay`
  (bind _keys (`BlueprintMapLibrary.Map_Keys` (`self.PathTable`)))
  (for _array_element _keys
    (if (`KismetArrayLibrary.Array_Contains` (`self.SelectedIndividuals`) _array_element)
      (bind _value (`BlueprintMapLibrary.Map_Find` (`self.PathTable`) _array_element))
      (bind _returnvalue (`|SpawnActorFromClass` "/Game/BP_PathEntity.BP_PathEntity_C" (`KismetMathLibrary.MakeTransform` (0.0 0.0 0.0)) "Undefined" "MultiplyWithRoot" null (break `/Game/S_PathEntity` _value) (`.Coordinates_6_645C3F94447EE674B4DA2BB01E27D0B6` (break `/Game/S_PathEntity` _value)) null))
      (`|SpawnActorFromClass` "/Game/BP_Penguin.BP_Penguin_C" (`KismetMathLibrary.MakeTransform` (0.0 0.0 0.0)) "AlwaysSpawn" "MultiplyWithRoot" null (break `/Game/S_PathEntity` _value) _returnvalue null))))

(fn `GPStoPosition`
  (params (Entry :type "/Game/S_PenguinGPS Structure (by ref)"))
  (returns (Position :type "Vector Structure"))
  (bind (_timestamp _location_long _location_lat) (break `/Game/S_PenguinGPS` Entry))
  (return (* (- (`KismetMathLibrary.MakeVector` _location_long _location_lat) (`self.PositionReference`)) (`self.PositionScale`))))

(fn `UserConstructionScript`
  (locals (TableNames :type "Array of Name") (TempTable :type "Array of Vector Structure"))
  (bind _parsefulltable (`self.ParseFullTable`))
  (`|ExecutionSequence`
    (:`then_0`
      (`BlueprintMapLibrary.Map_Clear` (`self.PathTable`))
      (`KismetArrayLibrary.Array_Clear` (`self.TempTable`))
      (`KismetArrayLibrary.Array_Clear` (`self.TableNames`)))
    (:`then_1`
      ;[1 1 1] Get Reference Position
      (bind _outrownames (`DataTableFunctionLibrary.GetDataTableRowNames` (`self.DataTable`)))
      (bind _output_get (set `local.TableNames` _outrownames))
      (bind _returnvalue (`|GetDataTableRow` (`self.DataTable`) (`|GetArrayItem` _output_get (`self.ReferenceRow`)))
        (:`then`
          (bind (_timestamp _location_long _location_lat) (break `/Game/S_PenguinGPS` _returnvalue))
          (set `self.PositionReference` (`KismetMathLibrary.MakeVector` _location_long _location_lat)))))
    (:`then_2`
      (for _index (range (`KismetMathLibrary.SelectInt` 0 (`self.MinTableIndex`) _parsefulltable) (+ (`KismetMathLibrary.SelectInt` (- (`KismetArrayLibrary.Array_Length` (`local.TableNames`)) 1) (`self.MaxTableIndex`) _parsefulltable) 1))
        (bind _returnvalue_2 (`|GetDataTableRow` (`self.DataTable`) (`|GetArrayItem` (`local.TableNames`) _index))
          (:`then`
            (bind _position (`self.GPStoPosition` _returnvalue_2))
            (bind ((`individual-local-identifier_12_9AC8A2A14EFFF01C7A5292B27DF39373` _individual_local_identifier)) (break `/Game/S_PenguinGPS` _returnvalue_2))
            (bind (_value _returnvalue_3) (`BlueprintMapLibrary.Map_Find` (`self.PathTable`) _individual_local_identifier))
            (if _returnvalue_3
              (bind _output_get_2 (set `local.TempTable` (`.Coordinates_6_645C3F94447EE674B4DA2BB01E27D0B6` (break `/Game/S_PathEntity` _value))))
              (`KismetArrayLibrary.Array_Add` _output_get_2 _position)
              (`BlueprintMapLibrary.Map_Add` (`self.PathTable`) _individual_local_identifier (make `/Game/S_PathEntity` (break `/Game/S_PathEntity` _value) (`local.TempTable`)))
              (else
                (bind _output_get_3 (set `local.TempTable` (`|MakeArray` _position)))
                (`BlueprintMapLibrary.Map_Add` (`self.PathTable`) _individual_local_identifier (make `/Game/S_PathEntity` (break `/Game/S_PathEntity` _value) _output_get_3))))))))))