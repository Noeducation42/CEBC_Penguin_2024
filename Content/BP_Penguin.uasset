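; Penguin actor with a sex and a family identity that travels along an assigned spline path.
; Construction scales the sphere mesh and collision by sex and tints a dynamic material blue for males or pink for females.
; Tick places it on the path by a speed-scaled time at constant spline velocity, without sweeping.
; BeginPlay prints males' children for debugging; overlap events are empty.
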(event `self.ReceiveBeginPlay`
  (bind (_identity_sex _identity_age _identity_size _identity_partner _identity_children) (break `/Game/S_Penguin` (`self.Identity`)))
  (`|ExecutionSequence`
    (:`then_1`
      (if (`|EnumEquality` (`self.Sex`) "NewEnumerator0")
        (for (_array_element _array_index) _identity_children
          (`KismetSystemLibrary.PrintString` (`KismetStringLibrary.Concat_StrStr` (`KismetStringLibrary.Conv_IntToString` _array_index) ": " (`KismetSystemLibrary.GetObjectName` _array_element)) true false (struct :`R` 1.0 :`B` 0.808595 :`A` 1.0) 60.0))))))

(event `self.ReceiveActorBeginOverlap`
  (params (OtherActor :type "Actor Object Reference")))

(event `self.ReceiveTick`
  (params (DeltaSeconds :type "Float (single-precision)"))
  (bind _path (`self.Path`))
  (`|ExecutionSequence`
    (:`then_1`
      (`/Engine/EditorBlueprintResources/StandardMacros.IsValid` _path
        (:`Is Valid`
          (`self.K2_SetActorLocation` (`SplineComponent.GetLocationAtTime` (`/Game/BP_PathEntity.Spline` _path) (`self.Time`) "World" true))
          (set `self.Time` (+ (`self.Time`) (* DeltaSeconds (`self.Speed`)))))))))

(event `self.Collision.OnComponentBeginOverlap`
  (params (OverlappedComponent :type "PrimitiveComponent Object Reference") (OtherActor :type "Actor Object Reference") (OtherComp :type "PrimitiveComponent Object Reference") (OtherBodyIndex :type Integer) (bFromSweep :type Boolean) (SweepResult :type "HitResult Structure (by ref)")))

(fn `UserConstructionScript`
  (locals (CollisionScale :type "Float (double-precision)" :default 3.0))
  (bind _femalesize (`self.FemaleSize`))
  (bind _collision_scale (`self.Collision Scale`))
  (bind _malesize (`self.MaleSize`))
  (bind _returnvalue (* _femalesize 0.5))
  (bind _returnvalue_2 (* _malesize 0.5))
  (bind _returnvalue_3 (select `/Game/E_Sex` (`self.Sex`) :`NewEnumerator0` (`KismetMathLibrary.MakeVector` _returnvalue_2 _returnvalue_2 _malesize) :`NewEnumerator1` (`KismetMathLibrary.MakeVector` _returnvalue _returnvalue _femalesize)))
  ;[1 0.7344 0.7344] Scale
  (`SceneComponent.SetWorldScale3D` (`self.Sphere`) _returnvalue_3)
  (`SceneComponent.SetWorldScale3D` (`self.Collision`) (* _returnvalue_3 (`KismetMathLibrary.MakeVector` _collision_scale _collision_scale _collision_scale)))
  ;[1 1 1] Material
  (bind _returnvalue_4 (`PrimitiveComponent.CreateDynamicMaterialInstance` (`self.Sphere`) 0 "/Game/M_SimpleColor.M_SimpleColor" "None"))
  (`MaterialInstanceDynamic.SetVectorParameterValue` _returnvalue_4 "BaseColor" (select `/Game/E_Sex` (`self.Sex`) :`NewEnumerator0` (struct :`R` 0.165314 :`G` 0.169168 :`B` 1.0 :`A` 1.0) :`NewEnumerator1` (struct :`R` 1.0 :`G` 0.430247 :`B` 0.755682 :`A` 1.0) :!type "LinearColor Structure"))
  (`PrimitiveComponent.SetMaterial` (`self.Sphere`) 0 _returnvalue_4))