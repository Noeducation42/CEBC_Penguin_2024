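; BP_PenguinPath draws a penguin's path from PathList as a colored tube, built entirely in the construction script.
; Each entry adds a spline point with an up vector from its rotation, then non-colliding, shadowless spline meshes span consecutive points, omitting the final segment.
; Dynamic materials color segments by depth through DepthColorCurve, or fixed teal where the point is flagged Generated.
; GetDataAt is an empty stub.
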(fn `GetDataAt`
  (params (Time :type "Float (double-precision)"))
  (returns (Data :type "/Game/S_PathData Structure")))

(fn `UserConstructionScript`
  (locals (PrevPosition :type "Vector Structure"))
  (bind _spline (`self.Spline`))
  (bind _meshscale (`self.MeshScale`))
  (bind _meshscale_2 (`self.MeshScale`))
  (bind _spline_2 (`self.Spline`))
  (`|ExecutionSequence`
    (:`then_0`
      ;[1 1 1] Init scale
      (set `self.MeshScale` (* (`self.UnitScale`) (`self.MeshWidth`) 0.0001)))
    (:`then_1`
      ;[1 1 1] Generate spline
      (for (_array_element _array_index) (`self.PathList`)
        (bind (_position _rotation) (break `/Game/S_PathData` _array_element))
        (`SplineComponent.AddSplinePointAtIndex` (`self.Spline`) _position _array_index "World" false)
        (`SplineComponent.SetUpVectorAtSplinePoint` (`self.Spline`) _array_index (`KismetMathLibrary.GetUpVector` _rotation) "Local" false))
      (`SplineComponent.UpdateSpline` (`self.Spline`)))
    (:`then_2`
      (for _index (range (+ (- (`SplineComponent.GetNumberOfSplinePoints` (`self.Spline`)) 3) 1))
        (bind _returnvalue (`AddComponent|NODE_AddSplineMeshComponent-0`))
        (`StaticMeshComponent.SetStaticMesh` _returnvalue (`self.Mesh`))
        (bind _returnvalue_2 (`PrimitiveComponent.CreateDynamicMaterialInstance` _returnvalue 0 "/Game/M_SimpleColor.M_SimpleColor" "None"))
        (bind (_returnvalue_x _returnvalue_y _returnvalue_z) (`KismetMathLibrary.BreakVector` (`SplineComponent.GetLocationAtSplinePoint` (`self.Spline`) _index "World")))
        (bind (_output_position _output_rotation _output_generated) (break `/Game/S_PathData` (`|GetArrayItem` (`self.PathList`) _index)))
        (`MaterialInstanceDynamic.SetVectorParameterValue` _returnvalue_2 "BaseColor" (`KismetMathLibrary.SelectColor` (struct :`R` 0.167958 :`G` 0.478099 :`B` 0.5 :`A` 1.0) (`CurveLinearColor.GetLinearColorValue` (`self.DepthColorCurve`) (`KismetMathLibrary.MapRangeClamped` (/ _returnvalue_z (`self.UnitScale`)) 0.0 -60.0 0.0 1.0)) _output_generated))
        (`PrimitiveComponent.SetCollisionEnabled` _returnvalue "NoCollision")
        (`PrimitiveComponent.SetCastShadow` _returnvalue false)
        (`SplineMeshComponent.SetForwardAxis` _returnvalue "Z" false)
        (bind _returnvalue_3 (+ _index 1))
        (`SplineMeshComponent.SetStartAndEnd` _returnvalue (`SplineComponent.GetLocationAtSplinePoint` _spline _index "World") (`SplineComponent.GetTangentAtSplinePoint` _spline _index "World") (`SplineComponent.GetLocationAtSplinePoint` _spline_2 _returnvalue_3 "World") (`SplineComponent.GetTangentAtSplinePoint` _spline_2 _returnvalue_3 "World") false)
        (`SplineMeshComponent.SetStartScale` _returnvalue (`KismetMathLibrary.MakeVector2D` _meshscale_2 _meshscale_2) false)
        (`SplineMeshComponent.SetEndScale` _returnvalue (`KismetMathLibrary.MakeVector2D` _meshscale _meshscale) true)))))