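; BP_PathEntity is a path Blueprint that builds a spline from its Coordinates array.
; The Construction Script appends each coordinate as a world-space Curve point, deferring the spline update until all points are added, without clearing existing points.
; A separate GPStoPosition helper swaps X and Y, flattens Z, then offsets and scales by PositionReference and PositionScale; nothing here calls it.
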(event `self.ReceiveBeginPlay`)

(fn `GPStoPosition`
  (params (Entry :type "/Game/S_PenguinGPS Structure (by ref)"))
  (returns (Position :type "Vector Structure"))
  (bind (_altitude _x _y) (break `/Game/S_PenguinGPS` Entry))
  (return (* (- (`KismetMathLibrary.MakeVector` _y _x) (`self.PositionReference`)) (`self.PositionScale`))))

(fn `UserConstructionScript`
  (locals (TableNames :type "Array of Name"))
  (bind _spline (`self.Spline`))
  (`|ExecutionSequence`
    (:`then_0`
      (for _array_element (`self.Coordinates`)
        (`SplineComponent.AddSplinePoint` _spline _array_element "World" false)
        (`SplineComponent.SetSplinePointType` (`self.Spline`) (- (`SplineComponent.GetNumberOfSplinePoints` _spline) 1) "Curve" false)))
    (:`then_2`
      (`SplineComponent.UpdateSpline` (`self.Spline`)))))