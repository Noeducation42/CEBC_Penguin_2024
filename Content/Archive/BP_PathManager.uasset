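; BP_PathManager turns GPS tracking rows from a DataTable into a path and spawns a penguin to follow it.
; The construction script converts rows to scaled positions relative to a reference row, with roll and pitch, dropping points closer than a minimum distance to the last kept one.
; BeginPlay spawns BP_PenguinPath from that table, passes it to a new BP_Penguin, and prints spline debug info.
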(event `self.ReceiveBeginPlay`
  (bind _returnvalue (`|SpawnActorFromClass` "/Game/BP_PenguinPath.BP_PenguinPath_C" (`KismetMathLibrary.MakeTransform` (0.0 0.0 0.0)) "Undefined" "MultiplyWithRoot" null (`self.PathTable`) "/Engine/BasicShapes/Cylinder.Cylinder" (`self.PositionScale`) 20.0 null))
  (`|SpawnActorFromClass` "/Game/BP_Penguin.BP_Penguin_C" (`KismetMathLibrary.MakeTransform` (0.0 0.0 0.0)) "Undefined" "MultiplyWithRoot" null "None" _returnvalue (/ (`self.PositionScale`) 100.0) 0.0001 null)
  (bind _spline (`/Game/BP_PenguinPath.Spline` _returnvalue))
  (bind _returnvalue_2 (`SplineComponent.GetSplineLength` _spline))
  (`KismetSystemLibrary.PrintString` (`KismetStringLibrary.Conv_DoubleToString` _returnvalue_2) true true (struct :`G` 0.66 :`B` 1.0 :`A` 1.0) 9999.0)
  (`KismetSystemLibrary.PrintString` (`KismetStringLibrary.Conv_IntToString` (`SplineComponent.GetNumberOfSplinePoints` _spline)) true true (struct :`G` 0.66 :`B` 1.0 :`A` 1.0) 9999.0)
  (`KismetSystemLibrary.PrintString` (`KismetStringLibrary.Conv_DoubleToString` (`SplineComponent.GetTimeAtDistanceAlongSpline` _spline _returnvalue_2)) true true (struct :`G` 0.66 :`B` 1.0 :`A` 1.0) 9999.0))

(fn `GPStoPosition`
  (params (Entry :type "/Game/S_PenguinGPS Structure (by ref)"))
  (returns (Position :type "Vector Structure") (Rotation :type "Rotator Structure"))
  (bind (_altitude _x _y _day _time_seconds _pitch _roll) (break `/Game/S_PenguinGPS` Entry))
  (bind (_returnvalue_x _returnvalue_y) (`KismetMathLibrary.BreakVector` (* (- (`KismetMathLibrary.MakeVector` _y _x) (`self.PositionReference`)) (`self.PositionScale`))))
  (return (`KismetMathLibrary.MakeVector` _returnvalue_x _returnvalue_y (* (`self.PositionScale`) _altitude)) (`KismetMathLibrary.MakeRotator` _roll _pitch)))

(fn `UserConstructionScript`
  (locals (TableNames :type "Array of Name") (TempTable :type "Array of Vector Structure") (PreviousPosition :type "Vector Structure" :default (0.0 0.0 0.0)))
  (bind _parsefulltable (`self.ParseFullTable`))
  (`|ExecutionSequence`
    (:`then_0`
      ;[1 1 1] Clear tables
      (`KismetArrayLibrary.Array_Clear` (`self.TableNames`))
      (`KismetArrayLibrary.Array_Clear` (`self.PathTable`)))
    (:`then_1`
      ;[1 1 1] Get Reference Position
      (bind _outrownames (`DataTableFunctionLibrary.GetDataTableRowNames` (`self.DataTable`)))
      (bind _output_get (set `local.TableNames` _outrownames))
      (bind _returnvalue (`|GetDataTableRow` (`self.DataTable`) (`|GetArrayItem` _output_get (`self.ReferenceRow`)))
        (:`then`
          (bind (_altitude _x _y) (break `/Game/S_PenguinGPS` _returnvalue))
          (set `self.PositionReference` (`KismetMathLibrary.MakeVector` _y _x)))))
    (:`then_2`
      (set `local.PreviousPosition` (0.0 0.0 0.0))
      (for _index (range (`KismetMathLibrary.SelectInt` 0 (`self.MinTableIndex`) _parsefulltable) (+ (`KismetMathLibrary.SelectInt` (- (`KismetArrayLibrary.Array_Length` (`local.TableNames`)) 1) (`self.MaxTableIndex`) _parsefulltable) 1))
        (bind _returnvalue_2 (`|GetDataTableRow` (`self.DataTable`) (`|GetArrayItem` (`local.TableNames`) _index))
          (:`then`
            (bind (_position _rotation) (`self.GPStoPosition` _returnvalue_2))
            (if (> (`KismetMathLibrary.Vector_Distance` _position (`local.PreviousPosition`)) (`self.MinDistance`))
              (`KismetArrayLibrary.Array_Add` (`self.PathTable`) (make `/Game/S_PathData` _position _rotation (`.Generated_39_E9B6907446850397BAF161B9E7342B18` (break `/Game/S_PenguinGPS` _returnvalue_2))))
              (set `local.PreviousPosition` _position))))))))