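; Penguin actor that moves along an assigned Path spline, with a Sex and an Identity holding family links.
; Tick advances a Time counter by Speed, samples the spline for location, roll and yaw, and shows the time on TimeText.
; Construction applies uniform Scale, and males print their children's names on BeginPlay for debugging.
; Sex-based sizing, coloring and partner movement remain as disconnected, unused logic.
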(event `self.ReceiveBeginPlay`
  (bind (_identity_sex _identity_age _identity_size _identity_partner _identity_children) (break `/Game/S_Penguin` (`self.Identity`)))
  (`|ExecutionSequence`
    (:`then_1`
      (if (`|EnumEquality` (`self.Sex`) "NewEnumerator0")
        (for (_array_element _array_index) _identity_children
          (`KismetSystemLibrary.PrintString` (`KismetStringLibrary.Concat_StrStr` (`KismetStringLibrary.Conv_IntToString` _array_index) ": " (`KismetSystemLibrary.GetObjectName` _array_element)) true false (struct :`R` 1.0 :`B` 0.808595 :`A` 1.0) 60.0))))))

(event `self.ReceiveActorBeginOverlap`
  (params (OtherActor :type "Actor Object Reference")))

(event `self.ReceiveTick`
  (params (DeltaSeconds :type "Float (single-precision)"))
  (bind _scale (`self.Scale`))
  (bind _path (`self.Path`))
  (bind _returnvalue (`SplineComponent.GetTransformAtTime` (`/Game/BP_PenguinPath.Spline` _path) (`self.Time`) "World" false false))
  (`|ExecutionSequence`
    (:`then_1`
      ;[1 1 1] Adjust the pinguin to the spline
      (`/Engine/EditorBlueprintResources/StandardMacros.IsValid` _path
        (:`Is Valid`
          (`self.K2_SetActorTransform` (`KismetMathLibrary.MakeTransform` (.location _returnvalue) (`KismetMathLibrary.MakeRotator` (.roll (.rotation _returnvalue)) 0.0 (.yaw (.rotation _returnvalue))) (`KismetMathLibrary.MakeVector` _scale _scale _scale)))
          ;[1 1 1] Increment timer
          (bind _output_get (set `self.Time` (+ (`self.Time`) (* DeltaSeconds (`self.Speed`)))))
          (`TextRenderComponent.K2_SetText` (`self.TimeText`) (`KismetTextLibrary.Conv_DoubleToText` _output_get "HalfToEven")))))))

(fn `UserConstructionScript`
  (locals (CollisionScale :type "Float (double-precision)" :default 3.0))
  (bind _scale (`self.Scale`))
  (`self.SetActorScale3D` (`KismetMathLibrary.MakeVector` _scale _scale _scale)))